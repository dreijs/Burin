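; BP_WorldSphere is a rotatable globe that displays the Burin world map in selectable map modes.
; Initialize creates a render target and feeds it to a dynamic material on the sphere.
; Draw calls planned by the Burin world are drawn as terrain, domain and border triangles onto that canvas.
; Rotation incrementally renders the current view, while year or map mode changes clear and redraw it.
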(event Custom|OnYearChange
  (params (NewYear :type Integer))
  (CallFunction|ResetSphereRender)
  (CallFunction|RenderWorldSphere))

(event EventBeginPlay
  (EventDispatchers|BindEventtoOnCurrentYearChanged (Class|BurinWorldSubsystem|GetBurinWorld (Subsystems|GetBurinWorldSubsystem)) (delegate Custom|OnYearChange)))

(event Collision|EventActorBeginOverlap
  (params (OtherActor :type Actor%20Object%20Reference)))

(event EventTick
  (params (DeltaSeconds :type Float%20%28single-precision%29)))

(fn ConstructionScript)

(fn RotateWorldSphere
  (params (Up :type Float%20%28double-precision%29) (Right :type Float%20%28double-precision%29))
  (Variables|Default|SetcLat Up)
  (Variables|Default|SetcLon Right)
  (Transformation|SetActorRotation "0, 0, 0")
  (Transformation|AddActorLocalRotation (Math|Rotator|MakeRotator 0.0 (Variables|Default|GetcLat) 0.0) false false)
  (Transformation|AddActorLocalRotation (Math|Rotator|MakeRotator 0.0 0.0 (Variables|Default|GetcLon)) false false)
  (CallFunction|RenderWorldSphere))

(fn Initialize
  (Utilities|FlowControl|Sequence
    (:then_0
      (bind _returnvalue (Rendering|CreateRenderTarget2D (Variables|Default|GetWidth) (Variables|Default|GetHeight) "RTF_RGBA16f"))
      (Variables|Default|SetSphereRenderTarget _returnvalue)
      (CallFunction|ResetSphereRender))
    (:then_1
      (bind _returnvalue_2 (Rendering|Material|CreateDynamicMaterialInstance "/Game/Materials/MAT_WorldSphereCanvas.MAT_WorldSphereCanvas" "None" "None" :!class /Script/Engine.KismetMaterialLibrary))
      (Rendering|Material|SetTextureParameterValue _returnvalue_2 "WorldCanvasTexture" (Variables|Default|GetSphereRenderTarget))
      (Rendering|Material|SetMaterial (Variables|Components|GetSphere) 0 _returnvalue_2))))

(fn SetZoomLevel
  (params (ZoomLevel :type Integer) (ZoomCategory :type Integer))
  (Variables|Default|SetZoomLevel ZoomLevel)
  (Variables|Default|SetZoomCategory ZoomCategory))

(fn SetMapMode
  (params (MapMode :type Integer))
  (Variables|Default|SetMapMode MapMode)
  (CallFunction|ResetSphereRender)
  (CallFunction|RenderWorldSphere))

(fn RenderWorldSphere
  (bind _returnvalue (Class|BurinWorld|PlanDrawsforView (Class|BurinWorldSubsystem|GetBurinWorld (Subsystems|GetBurinWorldSubsystem)) (Variables|Default|GetMapMode) (Variables|Default|GetZoomCategory) (Variables|Default|GetcLat) (Variables|Default|GetcLon) 22.5 (Variables|Default|GetWidth) (Variables|Default|GetHeight)))
  (CallFunction|ProcessDrawCalls _returnvalue))

(fn ResetSphereRender
  (Rendering|ClearRenderTarget2D (Variables|Default|GetSphereRenderTarget) "(R=1.000000,G=1.000000,B=1.000000,A=1.000000)")
  (Class|BurinWorld|ResetMapCoverage (Class|BurinWorldSubsystem|GetBurinWorld (Subsystems|GetBurinWorldSubsystem)))
  (bind _returnvalue (Class|BurinWorld|PlanDraws (Class|BurinWorldSubsystem|GetBurinWorld (Subsystems|GetBurinWorldSubsystem)) (Variables|Default|GetMapMode) 0 0.0 0.0 0.0 0.0 (Variables|Default|GetWidth) (Variables|Default|GetHeight)))
  (CallFunction|ProcessDrawCalls _returnvalue))

(fn ProcessDrawCalls
  (params (Calls :type Array%20of%20Map%20Draw%20Call%20Structures))
  (bind _returnvalue (Subsystems|GetBurinWorldSubsystem))
  (bind _mapmode (Variables|Default|GetMapMode))
  (bind _returnvalue_2 (Class|BurinWorldSubsystem|GetBurinWorld _returnvalue))
  (if (> (Utilities|Array|Length Calls) 0)
    (bind (_canvas _size _context) (Rendering|BeginDrawCanvastoRenderTarget (Variables|Default|GetSphereRenderTarget)))
    (for _array_element Calls
      (Utilities|FlowControl|Sequence
        (:then_0
          (bind _returnvalue_3 (Class|BurinWorld|GetTerrainTrianglesforDrawCall _returnvalue_2 _mapmode _array_element))
          (Class|Canvas|DrawTriangle _canvas 0 _returnvalue_3))
        (:then_1
          (bind _returnvalue_4 (Class|BurinWorld|GetDomainTrianglesforDrawCall _returnvalue_2 _mapmode _array_element))
          (Class|Canvas|DrawTriangle _canvas 0 _returnvalue_4))
        (:then_2
          (bind _returnvalue_5 (Class|BurinWorld|GetBorderTrianglesforDrawCall _returnvalue_2 _mapmode _array_element 5.0))
          (Class|Canvas|DrawTriangle _canvas 0 _returnvalue_5))))
    (Rendering|EndDrawCanvastoRenderTarget _context)))