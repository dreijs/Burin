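; Player camera pawn for a zoomable world viewer that spawns the globe, atmosphere, clouds, flat map and HUD on BeginPlay.
; Zooming moves the camera exponentially closer, swapping globe for flat map past a threshold.
; WASD shifts latitude and longitude at zoom-scaled speed, rotating the globe or panning the map.
; Clicking the globe converts hit UVs to coordinates, querying BurinWorld for domain or terrain info shown in the HUD.
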(event Input|EnhancedActionEvents|EnhancedInputActionIA_ClickMapAction
  (params (ActionValue :type Float%20%28double-precision%29) (ElapsedSeconds :type Float%20%28double-precision%29) (TriggeredSeconds :type Float%20%28double-precision%29) (InputAction :type Input%20Action%20Object%20Reference :default "/Game/Inputs/Actions/IA_ClickMapAction.IA_ClickMapAction"))
  (bind _returnvalue (Game|GetPlayerController 0))
  (bind _returnvalue_2 (Subsystems|GetBurinWorldSubsystem))
  (bind _uihudvar (Variables|Default|GetUIHudVar))
  (bind _returnvalue_3 (Class|BurinWorldSubsystem|GetBurinWorld _returnvalue_2))
  (bind (_worldlocation _worlddirection) (Game|Player|ConvertMouseLocationToWorldSpace _returnvalue))
  (:Completed
    (bind _outhit (Collision|LineTraceByChannel _worldlocation (+ _worldlocation (* _worlddirection 1e+04)) "TraceTypeQuery1" true (Utilities|Array|MakeArray (Variables|Default|GetAtmosphereVar) (Variables|Default|GetCloudsVar)) "None"))
    (Utilities|Casting|CastToBP_WorldSphere (.HitActor (Collision|BreakHitResult _outhit)))
    (if (== (Variables|Default|GetMapMode) 7)
      (bind _returnvalue_4 (Class|BurinWorld|GetDomainatCoordinate _returnvalue_3 0 (* (+ (.X (Math|Vector2D|BreakVector2D (.UV (Class|GameplayStatics|FindCollisionUV _outhit)))) -0.5) 3.6e+02) (* (+ (.Y (Math|Vector2D|BreakVector2D (.UV (Class|GameplayStatics|FindCollisionUV _outhit)))) -0.5) 1.8e+02)))
      (Default|LoadDomainInfo _uihudvar _returnvalue_4)
      (else
        (bind _returnvalue_5 (Class|BurinWorld|GetTerrainDataatCoordinate _returnvalue_3 0 (* (+ (.X (Math|Vector2D|BreakVector2D (.UV (Class|GameplayStatics|FindCollisionUV _outhit)))) -0.5) 3.6e+02) (* (+ (.Y (Math|Vector2D|BreakVector2D (.UV (Class|GameplayStatics|FindCollisionUV _outhit)))) -0.5) 1.8e+02)))
        (bind _returnvalue_6 (Class|BurinWorld|GetTerrainText _returnvalue_3 _returnvalue_5))
        (bind _returnvalue_7 (Class|BurinWorld|GetTriangleIDatCoordinate _returnvalue_3 0 (* (+ (.X (Math|Vector2D|BreakVector2D (.UV (Class|GameplayStatics|FindCollisionUV _outhit)))) -0.5) 3.6e+02) (* (+ (.Y (Math|Vector2D|BreakVector2D (.UV (Class|GameplayStatics|FindCollisionUV _outhit)))) -0.5) 1.8e+02)))
        (Default|LoadTerrainInfo _uihudvar _returnvalue_5 _returnvalue_6 _returnvalue_7 (* (* (+ (.Y (Math|Vector2D|BreakVector2D (.UV (Class|GameplayStatics|FindCollisionUV _outhit)))) -0.5) 1.8e+02) -1.0) (* (+ (.X (Math|Vector2D|BreakVector2D (.UV (Class|GameplayStatics|FindCollisionUV _outhit)))) -0.5) 3.6e+02))))))

(event Input|EnhancedActionEvents|EnhancedInputActionIA_MoveWASDAction
  (params (ActionValue :type Vector%202D%20Structure) (ElapsedSeconds :type Float%20%28double-precision%29) (TriggeredSeconds :type Float%20%28double-precision%29) (InputAction :type Input%20Action%20Object%20Reference :default "/Game/Inputs/Actions/IA_MoveWASDAction.IA_MoveWASDAction"))
  (bind (_x _y) (Math|Vector2D|BreakVector2D ActionValue))
  (bind _currentzoomlevel (Variables|Default|GetCurrentZoomLevel))
  (bind _returnvalue (Math|Conversions|ToFloat(Integer) _currentzoomlevel))
  (bind _returnvalue_2 (Math|Float|Power 0.85 _returnvalue))
  (CallFunction|MoveorRotate (* _returnvalue_2 (* _x 0.5)) (* _returnvalue_2 (* _y 0.5))))

(event Input|EnhancedActionEvents|EnhancedInputActionIA_ZoomAction
  (params (ActionValue :type Float%20%28double-precision%29) (ElapsedSeconds :type Float%20%28double-precision%29) (TriggeredSeconds :type Float%20%28double-precision%29) (InputAction :type Input%20Action%20Object%20Reference :default "/Game/Inputs/Actions/IA_ZoomAction.IA_ZoomAction"))
  (CallFunction|UpdateWorldZoomLevel (Math|Float|Truncate ActionValue)))

(event Input|EnhancedActionEvents|EnhancedInputActionIA_SwitchMapAction
  (params (ActionValue :type Boolean) (ElapsedSeconds :type Float%20%28double-precision%29) (TriggeredSeconds :type Float%20%28double-precision%29) (InputAction :type Input%20Action%20Object%20Reference :default "/Game/Inputs/Actions/IA_SwitchMapAction.IA_SwitchMapAction"))
  (CallFunction|UpdateMapMode (Math|Integer|%(Integer) (+ 1 (Variables|Default|GetMapMode)) (Variables|Default|GetNumMapModes))))

(event EventBeginPlay
  (Utilities|FlowControl|Sequence
    (:then_0
      (Class|BurinWorld|Initialize (Class|BurinWorldSubsystem|GetBurinWorld (Subsystems|GetBurinWorldSubsystem))))
    (:then_1
      (bind _returnvalue (Game|SpawnActorfromClass "/Game/Blueprints/BP_WorldSphere.BP_WorldSphere_C" (Math|Transform|MakeTransform "510.000000,0.000000,0.000000" "0, 0, 0" "5.000000,5.000000,5.000000") "Undefined" "MultiplyWithRoot" 0 0))
      (Variables|Default|SetWorldSphereVar _returnvalue)
      (Default|Initialize _returnvalue)
      (bind _returnvalue_2 (Game|SpawnActorfromClass "/Game/Blueprints/BP_Atmosphere.BP_Atmosphere_C" (Math|Transform|MakeTransform "515.000000,0.000000,0.000000" "0, 0, 0" "5.000000,5.000000,5.000000") "Undefined" "MultiplyWithRoot" 0 0))
      (Variables|Default|SetAtmosphereVar _returnvalue_2)
      (bind _returnvalue_3 (Game|SpawnActorfromClass "/Game/Blueprints/BP_Clouds.BP_Clouds_C" (Math|Transform|MakeTransform "510.000000,0.000000,0.000000" "0, 0, 0" "5.000000,5.000000,5.000000") "Undefined" "MultiplyWithRoot" 0 0))
      (Variables|Default|SetCloudsVar _returnvalue_3)
      (Default|SetZoomLevel (Variables|Default|GetWorldSphereVar)))
    (:then_2
      (bind _returnvalue_4 (Game|SpawnActorfromClass "/Game/Blueprints/BP_WorldMap.BP_WorldMap_C" (Math|Transform|MakeTransform "0, 0, 0" "0, 0, 0" "1.000000,1.000000,1.000000") "Undefined" "MultiplyWithRoot" 0 0))
      (Variables|Default|SetWorldMapVar _returnvalue_4))
    (:then_3
      (bind _returnvalue_5 (UserInterface|CreateWidget "/Game/UI/UI_HUD.UI_HUD_C"))
      (bind _output_get (Variables|Default|SetUIHudVar _returnvalue_5))
      (UserInterface|Viewport|AddtoViewport _output_get 0)
      (Default|InitializeHud _returnvalue_5 (Class|BurinWorldSubsystem|GetBurinWorld (Subsystems|GetBurinWorldSubsystem)) (Variables|Default|GetWorldSphereVar))
      (Default|SetMapMode _returnvalue_5 (Variables|Default|GetMapMode)))
    (:then_4
      (CallFunction|UpdateWorldZoomLevel)
      (Default|RenderWorldSphere (Variables|Default|GetWorldSphereVar))
      (CallFunction|MoveorRotate 0.0 0.0))
    (:then_5
      (Variables|/Script/Engine.PlayerController|SetbShowMouseCursor (Game|GetPlayerController 0) true))))

(event Collision|EventActorBeginOverlap
  (params (OtherActor :type Actor%20Object%20Reference)))

(event EventTick
  (params (DeltaSeconds :type Float%20%28single-precision%29)))

(fn ConstructionScript)

(fn UpdateWorldZoomLevel
  (params (Update :type Integer))
  (bind _worldspherevar (Variables|Default|GetWorldSphereVar))
  (bind _worldmapvar (Variables|Default|GetWorldMapVar))
  (bind _output_get (Variables|Default|SetCurrentZoomLevel (Math|Integer|Min(Integer) (Math|Integer|Max(Integer) (+ Update (Variables|Default|GetCurrentZoomLevel))) 32)))
  (for (_array_element _array_index) (Variables|Default|GetZoomCategoryThresholds)
    (if (>= _output_get _array_element)
      (Variables|Default|SetCurrentZoomCategory (+ _array_index 1))))
  (Utilities|FlowControl|Sequence
    (:then_0
      (Development|PrintText (Utilities|Text|FormatText "zoom lvl/cat {x}, {y}" (Variables|Default|GetCurrentZoomLevel) (Variables|Default|GetCurrentZoomCategory))))
    (:then_1
      (Transformation|SetActorLocation (Math|Vector|MakeVector (select (>= (Variables|Default|GetCurrentZoomLevel) (Variables|Default|GetSphereOrPlaneThreshold)) 0.0 (* (Math|Float|Power 0.65 (Math|Conversions|ToFloat(Integer) (Variables|Default|GetCurrentZoomLevel))) -8e+02)) 0.0 0.0) false false))
    (:then_2
      (Rendering|SetActorHiddenInGame (Variables|Default|GetCloudsVar) (>= (Variables|Default|GetCurrentZoomLevel) 1)))
    (:then_3
      (Default|SetZoomLevel _worldspherevar (Variables|Default|GetCurrentZoomLevel) (Variables|Default|GetCurrentZoomCategory))
      (Rendering|SetActorHiddenInGame _worldspherevar (>= (Variables|Default|GetCurrentZoomLevel) (Variables|Default|GetSphereOrPlaneThreshold)))
      (Rendering|SetActorHiddenInGame (Variables|Default|GetAtmosphereVar) (>= (Variables|Default|GetCurrentZoomLevel) (Variables|Default|GetSphereOrPlaneThreshold))))
    (:then_4
      (Default|SetVisible _worldmapvar (>= (Variables|Default|GetCurrentZoomLevel) (Variables|Default|GetSphereOrPlaneThreshold)))
      (Default|SetZoomLevel _worldmapvar (Utilities|Operators|Subtract (Variables|Default|GetCurrentZoomLevel) (Variables|Default|GetSphereOrPlaneThreshold) 1) (Variables|Default|GetCurrentZoomCategory)))
    (:then_5
      (CallFunction|MoveorRotate 0.0 0.0))
    (:then_6
      (Default|SetMarkerZoom (Variables|Default|GetUIHudVar) (Variables|Default|GetCurrentZoomLevel) (>= (Variables|Default|GetCurrentZoomLevel) (Variables|Default|GetSphereOrPlaneThreshold))))))

(fn UpdateMapMode
  (params (NewMapMode :type Integer))
  (bind _output_get (Variables|Default|SetMapMode NewMapMode))
  (Utilities|FlowControl|Sequence
    (:then_0
      (if (<= (Variables|Default|GetCurrentZoomLevel) (Variables|Default|GetSphereOrPlaneThreshold))
        (Default|SetMapMode (Variables|Default|GetWorldSphereVar) _output_get)
        (else
          (Default|SetMapMode (Variables|Default|GetWorldMapVar) _output_get))))
    (:then_1
      (Default|SetMapMode (Variables|Default|GetUIHudVar) NewMapMode))))

(fn MoveorRotate
  (params (Up :type Float%20%28double-precision%29) (Right :type Float%20%28double-precision%29))
  (bind _worldspherevar (Variables|Default|GetWorldSphereVar))
  (bind _worldmapvar (Variables|Default|GetWorldMapVar))
  (bind _mapmode (Variables|Default|GetMapMode))
  (Variables|Default|SetcLongitude (+ Right (Variables|Default|GetcLongitude)))
  (if (> (+ Right (Variables|Default|GetcLongitude)) 1.8e+02)
    (Variables|Default|SetcLongitude (+ (+ Right (Variables|Default|GetcLongitude)) -3.6e+02)))
  (if (< (+ Right (Variables|Default|GetcLongitude)) -1.8e+02)
    (Variables|Default|SetcLongitude (+ (+ Right (Variables|Default|GetcLongitude)) 3.6e+02)))
  (Variables|Default|SetcLatitude (Math|Float|Min(Float) (Math|Float|Max(Float) (+ (Variables|Default|GetcLatitude) Up) -8e+01) 8e+01))
  (if (< (Variables|Default|GetCurrentZoomLevel) (Variables|Default|GetSphereOrPlaneThreshold))
    (Default|RotateWorldSphere _worldspherevar (Variables|Default|GetcLatitude) (Variables|Default|GetcLongitude))
    (Default|RotateClouds (Variables|Default|GetCloudsVar) (Variables|Default|GetcLatitude) (Variables|Default|GetcLongitude))
    (if (!= (Variables|/Game/Blueprints/BP_WorldSphere.BP_WorldSphere_C|GetMapMode _worldspherevar) _mapmode)
      (Default|SetMapMode _worldspherevar _mapmode)
      (Default|RenderWorldSphere _worldspherevar))
    (else
      (Utilities|FlowControl|Sequence
        (:then_0
          (if (!= (Variables|/Game/Blueprints/BP_WorldMap.BP_WorldMap_C|GetMapMode _worldmapvar) _mapmode)
            (Default|SetMapMode _worldmapvar _mapmode)
            (Default|RenderMap _worldmapvar)))
        (:then_1
          (Default|MoveMap _worldmapvar (Variables|Default|GetcLatitude) (Variables|Default|GetcLongitude))
          (Default|SetMarkerMapView (Variables|Default|GetUIHudVar) (Variables|Default|GetcLatitude) (Variables|Default|GetcLongitude) (Variables|/Game/Blueprints/BP_WorldMap.BP_WorldMap_C|GetMapOrigin _worldmapvar) (Variables|/Game/Blueprints/BP_WorldMap.BP_WorldMap_C|GetEastPerDegree _worldmapvar) (Variables|/Game/Blueprints/BP_WorldMap.BP_WorldMap_C|GetNorthPerDegree _worldmapvar)))))))