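; BP_PlayerCamera is the player's camera for viewing a world as a globe or a map, spawning BP_WorldSphere and BP_WorldMap at play start.
; WASD input rotates the sphere, with speed falling exponentially as zoom increases.
; Zoom input sets a clamped level that exponentially shortens the spring arm, hides clouds, and swaps the sphere for the map when close.
; A switch input cycles the map display mode rendered on the sphere.
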(event Input|EnhancedActionEvents|EnhancedInputActionIA_MoveWASDAction
  (params (ActionValue :type Vector%202D%20Structure) (ElapsedSeconds :type Float%20%28double-precision%29) (TriggeredSeconds :type Float%20%28double-precision%29) (InputAction :type Input%20Action%20Object%20Reference :default "/Game/Inputs/Actions/IA_MoveWASDAction.IA_MoveWASDAction"))
  (bind (_x _y) (Math|Vector2D|BreakVector2D ActionValue))
  (bind _worldspherevar (Variables|Default|GetWorldSphereVar))
  (bind _currentzoomlevel (Variables|Default|GetCurrentZoomLevel))
  (bind _returnvalue (Math|Conversions|ToFloat(Integer) _currentzoomlevel))
  (bind _returnvalue_2 (Math|Float|Power 0.85 _returnvalue))
  (:Triggered
    (Default|RotateWorldSphere _worldspherevar (* _returnvalue_2 (* _x 0.5)) (* _returnvalue_2 (* _y 0.5))))
  (:Completed
    (Default|RotateWorldSphere _worldspherevar 0.0 0.0)))

(event Input|EnhancedActionEvents|EnhancedInputActionIA_ZoomAction
  (params (ActionValue :type Float%20%28double-precision%29) (ElapsedSeconds :type Float%20%28double-precision%29) (TriggeredSeconds :type Float%20%28double-precision%29) (InputAction :type Input%20Action%20Object%20Reference :default "/Game/Inputs/Actions/IA_ZoomAction.IA_ZoomAction"))
  (CallFunction|UpdateWorldZoomLevel (Math|Float|Truncate ActionValue)))

(event Input|EnhancedActionEvents|EnhancedInputActionIA_SwitchMap
  (params (ActionValue :type Boolean) (ElapsedSeconds :type Float%20%28double-precision%29) (TriggeredSeconds :type Float%20%28double-precision%29) (InputAction :type Input%20Action%20Object%20Reference :default "/Game/Inputs/Actions/IA_SwitchMap.IA_SwitchMap"))
  (:Started
    (bind _output_get (Variables|Default|SetMapDisplayMode (Math|Integer|%(Integer) (+ 1 (Variables|Default|GetMapDisplayMode)) (Variables|Default|GetNumMapModes))))
    (Development|PrintString (Utilities|String|ToString(Integer) _output_get))
    (Default|RenderVcMapBP (Variables|Default|GetWorldSphereVar) _output_get)))

(event EventBeginPlay
  (Utilities|FlowControl|Sequence
    (:then_0
      (bind _returnvalue (Game|SpawnActorfromClass "/Game/Blueprints/BP_WorldSphere.BP_WorldSphere_C" (Math|Transform|MakeTransform "510.000000,0.000000,0.000000" "0, 0, 0" "5.000000,5.000000,5.000000") "Undefined" "MultiplyWithRoot" 0 0))
      (Variables|Default|SetWorldSphereVar _returnvalue))
    (:then_1
      (bind _returnvalue_2 (Game|SpawnActorfromClass "/Game/Blueprints/BP_WorldMap.BP_WorldMap_C" (Math|Transform|MakeTransform "510.000000,0.000000,0.000000" "0, 0, 0" "2.000000,2.000000,2.000000") "Undefined" "MultiplyWithRoot" 0 0))
      (Variables|Default|SetWorldMapVar _returnvalue_2)
      (Development|PrintText "Hello"))
    (:then_2
      (CallFunction|UpdateWorldZoomLevel))))

(event Collision|EventActorBeginOverlap
  (params (OtherActor :type Actor%20Object%20Reference)))

(event EventTick
  (params (DeltaSeconds :type Float%20%28single-precision%29)))

(fn ConstructionScript)

(fn UpdateWorldZoomLevel
  (params (Update :type Integer))
  (bind _output_get (Variables|Default|SetCurrentZoomLevel (Math|Integer|Min(Integer) (Math|Integer|Max(Integer) (+ Update (Variables|Default|GetCurrentZoomLevel))) 32)))
  (Utilities|FlowControl|Sequence
    (:then_0
      (Development|PrintString (Utilities|String|ToString(Integer) _output_get)))
    (:then_1
      (Variables|/Script/Engine.SpringArmComponent|SetTargetArmLength (Variables|Default|GetSpringArm) (* (Math|Float|Power 0.65 (Math|Conversions|ToFloat(Integer) (Variables|Default|GetCurrentZoomLevel))) 499.0)))
    (:then_2
      (Default|SetCloudsVisible (Variables|Default|GetWorldSphereVar) (<= (Variables|Default|GetCurrentZoomLevel) 1)))
    (:then_3
      (Rendering|SetActorHiddenInGame (Variables|Default|GetWorldSphereVar) (not (<= (Variables|Default|GetCurrentZoomLevel) 8)))
      (Rendering|SetActorHiddenInGame (Variables|Default|GetWorldMapVar) (<= (Variables|Default|GetCurrentZoomLevel) 8)))))