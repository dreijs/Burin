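; BP_WorldMap manages a scrollable, zoomable world map built from BP_WorldMapTile actors for the Burin world.
; MoveMap asks the Burin world which subregions are in view, spawns or destroys tiles to match, then repositions each using cosine-of-latitude longitude scaling.
; SetZoomLevel derives exponential zoom, degree scale and origin, passing the zoom level to tiles.
; Tiles re-render when the map mode or current world year changes, and can be hidden together.
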(event Custom|OnYearChange
  (params (NewYear :type Integer))
  (CallFunction|RenderMap))

(event EventBeginPlay
  (EventDispatchers|BindEventtoOnCurrentYearChanged (Class|BurinWorldSubsystem|GetBurinWorld (Subsystems|GetBurinWorldSubsystem)) (delegate Custom|OnYearChange)))

(event Collision|EventActorBeginOverlap
  (params (OtherActor :type Actor%20Object%20Reference)))

(event EventTick
  (params (DeltaSeconds :type Float%20%28single-precision%29)))

(fn ConstructionScript)

(fn MoveMap
  (params (Latitude :type Float%20%28double-precision%29) (Longitude :type Float%20%28double-precision%29))
  (bind _returnvalue (Math|Trig|Cos(Degrees) Latitude))
  (bind _unitsperdegree (Variables|Default|GetUnitsPerDegree))
  (bind _output_get (Variables|Default|SetMercatorFactor _returnvalue))
  (bind _output_get_2 (Variables|Default|SetEastPerDegree (Math|Vector|MakeVector 0.0 (* _returnvalue _unitsperdegree) 0.0)))
  (bind _output_get_3 (Variables|Default|SetNorthPerDegree (Math|Vector|MakeVector 0.0 0.0 _unitsperdegree)))
  (CallFunction|CheckTiles Latitude Longitude)
  (for _array_element (Variables|Default|GetWorldMapTiles)
    (Default|MoveTile _array_element Latitude Longitude (Variables|Default|GetZoomFactor) _output_get (Variables|Default|GetMapOrigin) _output_get_2 _output_get_3)))

(fn RenderMap
  (for _array_element (Variables|Default|GetWorldMapTiles)
    (Default|RenderTile _array_element (Variables|Default|GetMapMode))))

(fn CheckTiles
  (params (Latitude :type Float%20%28double-precision%29) (Longitude :type Float%20%28double-precision%29))
  (bind _worldmaptiles (Variables|Default|GetWorldMapTiles))
  (bind _returnvalue (Class|BurinWorld|GetSubregionIndicesforView (Class|BurinWorldSubsystem|GetBurinWorld (Subsystems|GetBurinWorldSubsystem)) (Variables|Default|GetZoomCategory) Latitude Longitude 22.5))
  (if (Math|Boolean|ORBoolean (!= (Variables|Default|GetMinX) (Utilities|Array|Get(acopy) _returnvalue)) (!= (Variables|Default|GetMinY) (Utilities|Array|Get(acopy) _returnvalue 1)) (!= (Variables|Default|GetMaxX) (Utilities|Array|Get(acopy) _returnvalue 2)) (!= (Variables|Default|GetMaxY) (Utilities|Array|Get(acopy) _returnvalue 3)))
    (Utilities|FlowControl|Sequence
      (:then_0
        (Variables|Default|SetMinX (Utilities|Array|Get(acopy) _returnvalue))
        (Variables|Default|SetMinY (Utilities|Array|Get(acopy) _returnvalue 1))
        (Variables|Default|SetMaxX (Utilities|Array|Get(acopy) _returnvalue 2))
        (Variables|Default|SetMaxY (Utilities|Array|Get(acopy) _returnvalue 3)))
      (:then_1
        (bind (_arrayindex _arrayelement) (Utilities|Array|ReverseforEachLoop _worldmaptiles)
          (:LoopBody
            (if (Math|Boolean|ORBoolean (< (Variables|/Game/Blueprints/BP_WorldMapTile.BP_WorldMapTile_C|GetSubregionX _arrayelement) (Variables|Default|GetMinX)) (> (Variables|/Game/Blueprints/BP_WorldMapTile.BP_WorldMapTile_C|GetSubregionX _arrayelement) (Variables|Default|GetMaxX)) (< (Variables|/Game/Blueprints/BP_WorldMapTile.BP_WorldMapTile_C|GetSubregionY _arrayelement) (Variables|Default|GetMinY)) (> (Variables|/Game/Blueprints/BP_WorldMapTile.BP_WorldMapTile_C|GetSubregionY _arrayelement) (Variables|Default|GetMaxY)))
              (Development|PrintText (Utilities|Text|FormatText "Remove {X} {Y}" (Variables|/Game/Blueprints/BP_WorldMapTile.BP_WorldMapTile_C|GetSubregionX _arrayelement) (Variables|/Game/Blueprints/BP_WorldMapTile.BP_WorldMapTile_C|GetSubregionY _arrayelement)))
              (Actor|DestroyActor _arrayelement)
              (Utilities|Array|RemoveIndex _worldmaptiles _arrayindex)))))
      (:then_2
        (for _index (range (Variables|Default|GetMinX) (Variables|Default|GetMaxX))
          (for _index_2 (range (Variables|Default|GetMinY) (Variables|Default|GetMaxY))
            (LocalVariables|SetTileExists false)
            (bind _array_element (Utilities|Array|ForEachLoopwithBreak (Variables|Default|GetWorldMapTiles) :!label _label)
              (:LoopBody
                (if (Math|Boolean|ANDBoolean (== (Variables|/Game/Blueprints/BP_WorldMapTile.BP_WorldMapTile_C|GetSubregionX _array_element) _index) (== (Variables|/Game/Blueprints/BP_WorldMapTile.BP_WorldMapTile_C|GetSubregionX _array_element) _index) (== (Variables|/Game/Blueprints/BP_WorldMapTile.BP_WorldMapTile_C|GetSubregionY _array_element) _index_2) (== (Variables|/Game/Blueprints/BP_WorldMapTile.BP_WorldMapTile_C|GetSubregionY _array_element) _index_2))
                  (LocalVariables|SetTileExists true)
                  (goto _label Break)))
              (:Completed
                (if (not (LocalVariables|GetTileExists))
                  (bind _returnvalue_2 (Game|SpawnActorfromClass "/Game/Blueprints/BP_WorldMapTile.BP_WorldMapTile_C" (Math|Transform|MakeTransform "510.000000,0.000000,0.000000" "0, 0, 0" "2.000000,2.000000,2.000000") "Undefined" "MultiplyWithRoot" 0 0))
                  (Default|Initialize _returnvalue_2 _index _index_2 (Variables|Default|GetNumSubregionsX) (Variables|Default|GetNumSubregionsY) (Variables|Default|GetZoomCategory))
                  (Utilities|Array|Add (Variables|Default|GetWorldMapTiles) _returnvalue_2)
                  (Development|PrintText (Utilities|Text|FormatText "Create: {X}, {Y}: {Z} existing" _index _index_2 (Utilities|Array|Length (Variables|Default|GetWorldMapTiles))))
                  (Default|RenderTile _returnvalue_2 (Variables|Default|GetMapMode))))))
          (Development|PrintText (Utilities|Text|FormatText "Num: {N}" (Utilities|Array|Length (Variables|Default|GetWorldMapTiles))))))
      (:then_3
        (Development|PrintText (Utilities|Text|FormatText "Subregion: {X}, {Y}, {Z}, {ZZ}" (Utilities|Array|Get(acopy) _returnvalue) (Utilities|Array|Get(acopy) _returnvalue 1) (Utilities|Array|Get(acopy) _returnvalue 2) (Utilities|Array|Get(acopy) _returnvalue 3)))
        (CallFunction|SetZoomLevel (Variables|Default|GetZoomLevel) (Variables|Default|GetZoomCategory))))))

(fn SetVisible
  (params (Visible :type Boolean))
  (for _array_element (Variables|Default|GetWorldMapTiles)
    (Rendering|SetActorHiddenInGame _array_element (not Visible))))

(fn SetZoomLevel
  (params (ZoomLevel :type Integer) (ZoomCategory :type Integer))
  (bind _returnvalue (Subsystems|GetBurinWorldSubsystem))
  (bind _returnvalue_2 (Class|BurinWorldSubsystem|GetBurinWorld _returnvalue))
  (for _array_element (Variables|Default|GetWorldMapTiles)
    (Variables|/Game/Blueprints/BP_WorldMapTile.BP_WorldMapTile_C|SetZoomLevel _array_element ZoomLevel))
  (Variables|Default|SetZoomLevel ZoomLevel)
  (Variables|Default|SetZoomCategory ZoomCategory)
  (bind _returnvalue_3 (Class|BurinWorld|GetNumSubregions _returnvalue_2 ZoomCategory true))
  (bind _returnvalue_4 (Class|BurinWorld|GetNumSubregions _returnvalue_2 ZoomCategory false))
  (Variables|Default|SetNumSubregionsX _returnvalue_3)
  (Variables|Default|SetNumSubregionsY _returnvalue_4)
  (Variables|Default|SetZoomFactor (* (Math|Float|Power 1.5 (Math|Conversions|ToFloat(Integer) ZoomLevel)) 15.0))
  (Variables|Default|SetUnitsPerDegree (/ (* (Variables|Default|GetTileDist) (Variables|Default|GetZoomFactor)) (/ 1.8e+02 (Math|Conversions|ToFloat(Integer) (Variables|Default|GetNumSubregionsY)))))
  (Variables|Default|SetMapOrigin (+ (Transformation|GetActorLocation) "500.000000,0.000000,0.000000")))

(fn SetMapMode
  (params (MapMode :type Integer))
  (Variables|Default|SetMapMode MapMode)
  (CallFunction|RenderMap))