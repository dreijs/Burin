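; BP_WorldMapTile is one tile of the world map, a plane showing a render target through a dynamic canvas material.
; RenderTile draws terrain, domain and border triangles from the Burin world subsystem onto the render target for a given map mode, then prints a debug pixel.
; MoveTile scales the plane with zoom and a Mercator factor and positions it relative to the viewed latitude/longitude.
; Timelines drive the material's fade in and out.
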(event Custom|FadeOutEvent
  (bind _dynamicmaterial (Variables|Default|GetDynamicMaterial))
  (Rendering|Material|SetScalarParameterValue _dynamicmaterial "FadeLevel" 1.0 :!class /Script/Engine.MaterialInstanceDynamic)
  (bind _fadeouttrack (Timeline|FadeOutTimeline PlayFromStart)
    (:Update
      (Rendering|Material|SetScalarParameterValue _dynamicmaterial "FadeLevel" _fadeouttrack :!class /Script/Engine.MaterialInstanceDynamic))))

(event Custom|FadeInEvent
  (bind _dynamicmaterial (Variables|Default|GetDynamicMaterial))
  (Rendering|Material|SetScalarParameterValue _dynamicmaterial "FadeLevel" 0.0 :!class /Script/Engine.MaterialInstanceDynamic)
  (bind _fadeintrack (Timeline|FadeInTimeline PlayFromStart)
    (:Update
      (Rendering|Material|SetScalarParameterValue _dynamicmaterial "FadeLevel" _fadeintrack :!class /Script/Engine.MaterialInstanceDynamic))))

(event EventBeginPlay
  (Utilities|FlowControl|Sequence
    (:then_0
      (bind _returnvalue (Rendering|CreateRenderTarget2D 2048 2048 "RTF_RGBA16f"))
      (Variables|Default|SetWorldMapRenderTarget _returnvalue))
    (:then_1
      (bind _returnvalue_2 (Rendering|Material|CreateDynamicMaterialInstance "/Game/Materials/MAT_WorldMapCanvas.MAT_WorldMapCanvas" "None" "None" :!class /Script/Engine.KismetMaterialLibrary))
      (Rendering|Material|SetTextureParameterValue _returnvalue_2 "WorldCanvasTexture" (Variables|Default|GetWorldMapRenderTarget))
      (Rendering|Material|SetMaterial (Variables|Default|GetPlane) 0 _returnvalue_2)
      (Variables|Default|SetDynamicMaterial _returnvalue_2))))

(event Collision|EventActorBeginOverlap
  (params (OtherActor :type Actor%20Object%20Reference)))

(event EventTick
  (params (DeltaSeconds :type Float%20%28single-precision%29)))

(fn ConstructionScript)

(fn RenderTile
  (params (MapMode :type Integer))
  (bind _returnvalue (Subsystems|GetBurinWorldSubsystem))
  (bind _worldmaprendertarget (Variables|Default|GetWorldMapRenderTarget))
  (bind _returnvalue_2 (Class|BurinWorldSubsystem|GetBurinWorld _returnvalue))
  (Rendering|ClearRenderTarget2D _worldmaprendertarget "(R=0.526042,G=0.000000,B=0.000000,A=1.000000)")
  (bind _returnvalue_3 (Class|BurinWorld|MakeTileDrawCall _returnvalue_2 (Variables|Default|GetZoomCategory) (Variables|Default|GetSubregionX) (Variables|Default|GetSubregionY) 2048 2048))
  (bind (_canvas _size _context) (Rendering|BeginDrawCanvastoRenderTarget _worldmaprendertarget))
  (Utilities|FlowControl|Sequence
    (:then_0
      (bind _returnvalue_4 (Class|BurinWorld|GetTerrainTrianglesforDrawCall _returnvalue_2 MapMode _returnvalue_3))
      (Class|Canvas|DrawTriangle _canvas 0 _returnvalue_4))
    (:then_1
      (bind _returnvalue_5 (Class|BurinWorld|GetDomainTrianglesforDrawCall _returnvalue_2 MapMode _returnvalue_3))
      (Class|Canvas|DrawTriangle _canvas 0 _returnvalue_5))
    (:then_2
      (bind _returnvalue_6 (Class|BurinWorld|GetBorderTrianglesforDrawCall _returnvalue_2 MapMode _returnvalue_3 5.0))
      (Class|Canvas|DrawTriangle _canvas 0 _returnvalue_6))
    (:then_3
      (Rendering|EndDrawCanvastoRenderTarget _context)
      (bind _returnvalue_7 (Class|KismetRenderingLibrary|ReadRenderTargetPixel (Variables|Default|GetWorldMapRenderTarget) 1024 1024))
      (Development|PrintText (Utilities|Text|FormatText "tile {x}, {y} pixel: {r}, {g}, {b}, (alpha {a})" (Variables|Default|GetSubregionX) (Variables|Default|GetSubregionY) (.R (Math|Color|BreakColor _returnvalue_7)) (.G (Math|Color|BreakColor _returnvalue_7)) (.B (Math|Color|BreakColor _returnvalue_7)) (.A (Math|Color|BreakColor _returnvalue_7)))))))

(fn MoveTile
  (params (Latitude :type Float%20%28double-precision%29) (Longitude :type Float%20%28double-precision%29) (ZoomFactor :type Float%20%28double-precision%29) (MercatorFactor :type Float%20%28double-precision%29) (Origin :type Vector) (EastPerDegree :type Vector) (NorthPerDegree :type Vector))
  (bind _returnvalue (Subsystems|GetBurinWorldSubsystem))
  (bind _subregionx (Variables|Default|GetSubregionX))
  (bind _subregiony (Variables|Default|GetSubregionY))
  (bind _zoomcategory (Variables|Default|GetZoomCategory))
  (bind _returnvalue_2 (Class|BurinWorldSubsystem|GetBurinWorld _returnvalue))
  (bind (_latitude _longitude) (Class|BurinWorld|GetTileCentreCoordinate _returnvalue_2 _zoomcategory _subregionx _subregiony))
  (Transformation|SetWorldScale3D (Variables|Default|GetPlane) (Math|Vector|MakeVector (* ZoomFactor MercatorFactor) ZoomFactor ZoomFactor))
  (Transformation|SetActorLocation (+ Origin (* EastPerDegree (- _longitude Longitude)) (* NorthPerDegree (- _latitude Latitude))) false false)
  (Variables|Default|SetcLongitude Longitude)
  (Variables|Default|SetcLatitude Latitude))

(fn Initialize
  (params (SubregionX :type Integer) (SubregionY :type Integer) (NumSubregionsX :type Integer) (NumSubregionsY :type Integer) (ZoomCategory :type Integer))
  (Variables|Default|SetSubregionX SubregionX)
  (Variables|Default|SetSubregionY SubregionY)
  (Variables|Default|SetNumSubregionsX NumSubregionsX)
  (Variables|Default|SetNumSubregionsY NumSubregionsY)
  (Variables|Default|SetZoomCategory ZoomCategory))

(fn SetZoomScale
  (params (ZoomLevel :type Integer))
  (Variables|Default|SetZoomLevel ZoomLevel))

(fn UpdateLocation
  (Transformation|SetActorLocation (Math|Vector|MakeVector 5.1e+02 (Variables|Default|GetcLongitude) (Variables|Default|GetcLatitude)) false false))